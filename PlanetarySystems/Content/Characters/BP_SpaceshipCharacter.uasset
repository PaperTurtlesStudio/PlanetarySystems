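; Player spaceship character with physics-driven flight, steered through thrust, roll, turn and look-up input axes.
; Thrust blends the static mesh's velocity toward actor forward at a clamped speed, so zero input still drives it forward.
; Rotation inputs apply scaled torque to the capsule about the actor's forward, up and right axes.
; Tick applies torque opposing the capsule's angular velocity to stabilize rotation.
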(event EventBeginPlay)

(event Collision|EventActorBeginOverlap
  (params (OtherActor :type Actor%20Object%20Reference)))

(event EventTick
  (params (DeltaSeconds :type Float%20%28single-precision%29))
  ;[1 1 1] Rotation Stablization
  (Class|PrimitiveComponent|AddTorqueinDegrees (Variables|Default|GetCapsuleComponent) (/ (Math|Vector|NegateVector (Physics|GetPhysicsAngularVelocityinDegrees (Variables|Default|GetCapsuleComponent) "None")) 2e+01) "None" true))

(event Input|AxisEvents|InputAxisThrust
  (params (AxisValue :type Float%20%28single-precision%29))
  ;[1 1 1] Thrust
  (bind _returnvalue (Physics|GetPhysicsLinearVelocity (Variables|Default|GetStaticMesh) "None"))
  (Physics|SetPhysicsLinearVelocity (Variables|Default|GetStaticMesh) (Math|Vector|Lerp(Vector) _returnvalue (* (Transformation|GetActorForwardVector) (Math|Float|Clamp(Float) (* AxisValue 5e+03) 5e+03 1e+04)) 0.1) false "None"))

(event Input|AxisEvents|InputAxisRoll
  (params (AxisValue :type Float%20%28single-precision%29))
  (Class|PrimitiveComponent|AddTorqueinDegrees (Variables|Default|GetCapsuleComponent) (Math|Vector|Lerp(Vector) "0, 0, 0" (* (Transformation|GetActorForwardVector) (* AxisValue 1e+03)) 0.1) "None" true))

(event Input|AxisEvents|InputAxisTurn
  (params (AxisValue :type Float%20%28single-precision%29))
  (Class|PrimitiveComponent|AddTorqueinDegrees (Variables|Default|GetCapsuleComponent) (Math|Vector|Lerp(Vector) "0, 0, 0" (* (Transformation|GetActorUpVector) (* AxisValue 1e+03)) 0.1) "None" true))

(event Input|AxisEvents|InputAxisLookUp
  (params (AxisValue :type Float%20%28single-precision%29))
  (Class|PrimitiveComponent|AddTorqueinDegrees (Variables|Default|GetCapsuleComponent) (Math|Vector|Lerp(Vector) "0, 0, 0" (* (Transformation|GetActorRightVector) (* AxisValue 1e+03)) 0.1) "None" true))

(fn ConstructionScript)